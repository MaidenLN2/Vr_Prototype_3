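; Buoy rope actor that lays a mesh along an editable spline and bobs up and down.
; The construction script adds a spline mesh component for each spline segment, matching its local-space endpoints and tangents.
; On BeginPlay, an endless Delay loop offsets the whole actor up and back down every second in instant steps, without sweep or interpolation.
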(event `self.ReceiveBeginPlay`
  (`self.K2_AddActorLocalOffset` (0.0 0.0 10.0) :!label _label)
  (`KismetSystemLibrary.Delay` 1.0)
  (`self.K2_AddActorLocalOffset` (0.0 0.0 -10.0))
  (`KismetSystemLibrary.Delay` 1.0)
  (goto _label))

(fn `UserConstructionScript`
  (for _index (range (`SplineComponent.GetNumberOfSplineSegments` (`self.Spline`)))
    (bind _returnvalue (`AddComponent|NODE_AddSplineMeshComponent-0`))
    (bind (_location _tangent) (`SplineComponent.GetLocationAndTangentAtSplinePoint` (`self.Spline`) _index "Local"))
    (bind (_location_2 _tangent_2) (`SplineComponent.GetLocationAndTangentAtSplinePoint` (`self.Spline`) (+ _index 1) "Local"))
    (`SplineMeshComponent.SetStartAndEnd` _returnvalue _location _tangent _location_2 _tangent_2 true)))