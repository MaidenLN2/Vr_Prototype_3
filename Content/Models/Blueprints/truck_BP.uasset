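; Truck Blueprint that makes its two point lights flicker at random intervals.
; Tick feeds a Delay of a random whole number of seconds below 100, which works as a repeating timer because Delay ignores calls while pending.
; When it fires, chained short delays switch both lights off and on twice, leaving them lit.
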(event `self.ReceiveBeginPlay`)

(event `self.ReceiveTick`
  (params (DeltaSeconds :type "Float (single-precision)"))
  (`KismetSystemLibrary.Delay` (`KismetMathLibrary.Conv_IntToDouble` (`KismetMathLibrary.RandomInteger` 100)))
  (`SceneComponent.SetVisibility` (`self.PointLight`) false false)
  (`SceneComponent.SetVisibility` (`self.PointLight1`) false false)
  (`KismetSystemLibrary.Delay` 0.1)
  (`SceneComponent.SetVisibility` (`self.PointLight`) true false)
  (`SceneComponent.SetVisibility` (`self.PointLight1`) true false)
  (`KismetSystemLibrary.Delay` 0.1)
  (`SceneComponent.SetVisibility` (`self.PointLight`) false false)
  (`SceneComponent.SetVisibility` (`self.PointLight1`) false false)
  (`KismetSystemLibrary.Delay` 0.2)
  (`SceneComponent.SetVisibility` (`self.PointLight`) true false)
  (`SceneComponent.SetVisibility` (`self.PointLight1`) true false))

(fn `UserConstructionScript`)